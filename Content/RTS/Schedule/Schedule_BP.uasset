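; Schedule Blueprint that stores a replicated list of entries, each covering one or more hour timeslots, and serves lookups by hour.
; GetEntryAtTime scans every entry's timeslots and returns the first entry with a range containing the given hour, or an empty result if none matches.
; The Entries rep-notify fires the OnEntriesChanged dispatcher so listeners can react to replicated updates.
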(fn OnRepEntries
  (Default|CallOnEntriesChanged))

(fn GetEntries
  (return (Variables|Default|GetEntries)))

(fn GetEntryatTime
  (params (Hour :type Integer))
  (for _array_element (Variables|Default|GetEntries)
    (for _array_element_2 (Utilities|Struct|BreakScheduleEntry_F _array_element)
      (if (Class|CppBlueprintCallableStatics|InRange _array_element_2 Hour)
        (return _array_element))))
  (return ""))