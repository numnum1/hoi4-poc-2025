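; State blueprint for the RTS that holds a state's name, picture and owning nation.
; All three properties replicate with RepNotify, and each notify fires the shared OnInfoChanged dispatcher so listeners can refresh on any change.
; Simple getters expose the three values to other classes.
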(fn ConstructionScript)

(fn OnRepName
  (Default|CallOnInfoChanged))

(fn OnRepPicture
  (Default|CallOnInfoChanged))

(fn OnRepOwningNation
  (Default|CallOnInfoChanged))

(fn GetName
  (return (Variables|Default|GetName)))

(fn GetPicture
  (return (Variables|Default|GetPicture)))

(fn GetOwningNation
  (return (Variables|Default|GetOwningNation)))