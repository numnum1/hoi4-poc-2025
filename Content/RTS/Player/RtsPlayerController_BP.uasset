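; RTS player controller that relays player commands to the server: game speed, organization founding, controlled character and building construction.
; At BeginPlay it binds every State_BP click to an OnStateClicked dispatcher, which right-click also fires without a state.
; ControlledCharacter is replicated, with its OnRep broadcasting changes.
; Server events drive Time_BP, spawn and register buildings, and create organizations, linking founder and organization through a shared position GUID.
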(event Custom|Server_SetSpeed
  (params (NewSpeed :type Integer))
  ;[0.15 0.15 0.15 0.5] Set Speed
  (bind _returnvalue (Actor|GetActorOfClass "/Game/RTS/Time/Time_BP.Time_BP_C"))
  (Default|SetSpeed _returnvalue NewSpeed))

(event Custom|Server_FoundOrganization
  (params (Name :type Text) (Logo :type Slate%20Brush%20Structure) (InitialHeadOfNewOrganization :type Rts%20Character%20BP%20Object%20Reference))
  ;[0.15 0.15 0.15 0.5] Found Organization
  (Utilities|MakeOrg Name Logo InitialHeadOfNewOrganization))

(event Custom|HandleStateClicked
  (params (TouchedActor :type Actor%20Object%20Reference) (ButtonPressed :type Key%20Structure :default "None"))
  (Default|CallOnStateClicked (.AsState%20BP (Utilities|Casting|CastToState_BP TouchedActor))))

(event Custom|Server_ControlCharacter
  (params (ControlledCharacter :type Rts%20Character%20BP%20Object%20Reference))
  ;[0.15 0.15 0.15 0.5] For Testing
  (Variables|Default|SetControlledCharacter ControlledCharacter))

(event Custom|Server_CreateBuilding
  (params (Building :type Building%20BP%20Class%20Reference) (For :type Actor%20Object%20Reference) (InState :type State%20BP%20Object%20Reference))
  (bind _returnvalue (Game|SpawnActorfromClass Building (Math|Transform|MakeTransform "0, 0, 0" "0, 0, 0" "1.000000,1.000000,1.000000") "Undefined" "MultiplyWithRoot" 0 InState For 0))
  (Default|RegisterBuilding InState _returnvalue)
  (Audio|PlaySound2D "/Game/RTS/Common/UI/SFX/Resources/Sigge/start_construction.start_construction" 1.0 1.0 0.0 0 0))

(event EventBeginPlay
  (bind _outactors (Actor|GetAllActorsOfClass "/Game/RTS/State/State_BP.State_BP_C"))
  (for _array_element _outactors
    (EventDispatchers|AssignOnClicked _array_element (delegate Custom|HandleStateClicked))))

(event Input|MouseEvents|DebugKeyRightMouseButton
  (params (Key :type Key%20Structure :default "None") (ActionValue :type Input%20Action%20Value%20Structure))
  (:Pressed
    (Default|CallOnStateClicked)))

(fn ConstructionScript)

(fn OnRepControlledCharacter
  (Default|CallOnControlledCharacterChanged))

(fn SetControlledCharacter
  (params (ControlledCharacter :type Rts%20Character%20BP%20Object%20Reference))
  (Variables|Default|SetControlledCharacter ControlledCharacter))

(fn GetControlledCharacter
  (return (Variables|Default|GetControlledCharacter)))