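; Music player for the RTS player that plays 2D audio from a set of playlists, starting with a random one on BeginPlay.
; Switching playlists fades out the current sound and fades in the active one's audio, guarded for dedicated servers.
; TogglePause fades out and later spawns the audio afresh rather than resuming it.
; Getters expose playlists, selection and play state, and OnPlayingChanged signals playback updates.
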(event Custom|PlayNext
  (Utilities|FlowControl|Sequence
    (:then_0
      (bind _player (Variables|Default|GetPlayer)
        (:then
          (Audio|Components|Audio|FadeOut _player 2.0 0.0 "Linear" :!class /Script/Engine.AudioComponent)
          (Variables|Default|SetPlayer 0))
        (:else)))
    (:then_1
      (bind _returnvalue (Audio|SpawnSound2D (.Audio (Utilities|Struct|BreakPlaylist (Utilities|Array|Get(acopy) (Variables|Default|GetPlaylists) (Variables|Default|GetActive)))) 1.0 1.0 0.0 0))
      (bind _output_get (Variables|Default|SetPlayer _returnvalue))
      ;[0.15 0.15 0.15 0.5] Dedicated server should not try
      (Utilities|IsValid _output_get
        (:Is%20Valid
          (Audio|Components|Audio|FadeIn _output_get 5.0 1.0 0.0 "Linear" :!class /Script/Engine.AudioComponent)
          (Variables|Default|SetbPlaying true)
          (Default|CallOnPlayingChanged))))))

(event Custom|TogglePause
  (if (Variables|Default|GetbPlaying)
    (bind _player (Variables|Default|GetPlayer)
      (:then
        (Audio|Components|Audio|FadeOut _player 2.0 0.0 "Linear" :!class /Script/Engine.AudioComponent)
        (Variables|Default|SetPlayer 0)
        (Variables|Default|SetbPlaying false))
      (:else))
    (else
      (bind _returnvalue (Audio|SpawnSound2D (.Audio (Utilities|Struct|BreakPlaylist (Utilities|Array|Get(acopy) (Variables|Default|GetPlaylists) (Variables|Default|GetActive)))) 1.0 1.0 0.0 0))
      (bind _output_get (Variables|Default|SetPlayer _returnvalue))
      (Utilities|IsValid _output_get
        (:Is%20Valid
          (Audio|Components|Audio|FadeIn _output_get 5.0 1.0 0.0 "Linear" :!class /Script/Engine.AudioComponent)
          (Variables|Default|SetbPlaying true)))))
  (Default|CallOnPlayingChanged))

(event Custom|SetActivePlaylist
  (params (Active :type Integer))
  (Variables|Default|SetActive Active)
  (if (Variables|Default|GetbPlaying)
    (CallFunction|PlayNext)))

(event EventBeginPlay
  (Variables|Default|SetActive (.OutIndex (Utilities|Array|Random (Variables|Default|GetPlaylists))))
  (CallFunction|PlayNext))

(event EventEndPlay
  (params (EndPlayReason :type EEndPlayReason%20Enum :default "Destroyed"))
  (bind _player (Variables|Default|GetPlayer)
    (:then
      (Audio|Components|Audio|Stop _player)
      (Variables|Default|SetPlayer 0)
      (Variables|Default|SetbPlaying false)
      (Default|CallOnPlayingChanged))
    (:else)))

(fn GetPlaylists
  (return (Variables|Default|GetPlaylists)))

(fn IsPlaying
  (return (Variables|Default|GetbPlaying)))

(fn GetActive
  (return (Variables|Default|GetActive)))