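; RTS HUD implementation that sets up the player's HUD in an MVVM pattern and handles organization founding requests.
; On BeginPlay it creates the view widget, gives it a new view model with this HUD as its model, and binds the view model's create-organization event.
; CreateOrganization forwards name, logo and the controlled character as initial head to player controller 0's ServerFoundOrganization, a route marked as temporary.
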(event Custom|CreateOrganization
  (params (Name :type Text) (Logo :type Slate%20Brush%20Structure))
  (bind _returnvalue (Game|GetPlayerController 0))
  (bind _asrts_player_controller_bp (Utilities|Casting|CastToRtsPlayerController_BP _returnvalue))
  (Default|ServerFoundOrganization _asrts_player_controller_bp Name Logo (Default|GetControlledCharacter _asrts_player_controller_bp)))

(event EventBeginPlay
  (|CallParentFunction)
  (bind _returnvalue (UserInterface|CreateWidget "/Game/RTS/Player/HUD/Implementation/RtsHUD_V.RtsHUD_V_C" 0 0))
  (Variables|Default|SetWidget _returnvalue)
  (bind _returnvalue_2 (Game|ConstructObjectfromClass "/Game/RTS/Player/HUD/Implementation/RtsHUD_VM.RtsHUD_VM_C"))
  (Default|SetModel _returnvalue_2 self)
  (Variables|/Game/RTS/Player/HUD/Implementation/RtsHUD_V.RtsHUD_V_C|SetRtsHUD_VM (Variables|Default|GetWidget) _returnvalue_2)
  (UserInterface|Viewport|AddtoViewport _returnvalue 0)
  (EventDispatchers|BindEventtoOnCreateOrganization _returnvalue_2 (EventDispatchers|CreateEvent :!event Custom|CreateOrganization)))

(fn ConstructionScript
  (|CallParentFunction))