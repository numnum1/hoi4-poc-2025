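; RTS HUD Blueprint that creates the main HUD widget and relays its player actions to the server.
; BeginPlay builds a view model from itself and the map actor, hands it to the widget, and binds organization-creation and property-purchase events.
; Handlers call server functions on the RTS player controller to found organizations or create buildings, playing a construction sound for the latter.
; Tick fires an OnTick call every frame.
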(event Custom|CreateOrganization
  (params (Name :type Text) (Logo :type Slate%20Brush%20Structure))
  (bind _returnvalue (Game|GetPlayerController 0))
  (bind _asrts_player_controller_bp (Utilities|Casting|CastToRtsPlayerController_BP _returnvalue))
  (Default|ServerFoundOrganization _asrts_player_controller_bp Name Logo (Default|GetControlledCharacter _asrts_player_controller_bp)))

(event Custom|BuyProperty
  (params (Building :type Building%20BP%20Class%20Reference) (For :type Actor%20Object%20Reference) (InState :type State%20BP%20Object%20Reference))
  (Default|ServerCreateBuilding (.AsRts%20Player%20Controller%20BP (Utilities|Casting|CastToRtsPlayerController_BP (Game|GetPlayerController 0))) Building For InState)
  (Audio|PlaySound2D "/Game/RTS/Common/UI/SFX/Resources/Sigge/start_construction.start_construction" 1.0 1.0 0.0 0 0))

(event EventBeginPlay
  (|CallParentFunction)
  (bind _returnvalue (UserInterface|CreateWidget "/Game/RTS/Player/HUD/RtsHUD_V.RtsHUD_V_C" 0 0))
  (Variables|Default|SetWidget _returnvalue)
  (bind _returnvalue_2 (Actor|GetActorOfClass "/Game/RTS/Map/RtsMap_BP.RtsMap_BP_C"))
  (bind _returnvalue_3 (Game|ConstructObjectfromClass "/Game/RTS/Player/HUD/RtsHUD_VM.RtsHUD_VM_C" _returnvalue_2))
  (Default|SetModel _returnvalue_3 self)
  (Variables|/Game/RTS/Player/HUD/RtsHUD_V.RtsHUD_V_C|SetRtsHUD_VM (Variables|Default|GetWidget) _returnvalue_3)
  (UserInterface|Viewport|AddtoViewport _returnvalue 0)
  (EventDispatchers|BindEventtoCreateOrganization _returnvalue_3 (EventDispatchers|CreateEvent :!event Custom|CreateOrganization))
  (EventDispatchers|BindEventtoBuyPropery _returnvalue_3 (EventDispatchers|CreateEvent :!event Custom|BuyProperty)))

(event EventTick
  (params (DeltaSeconds :type Float%20%28single-precision%29))
  (Default|CallOnTick DeltaSeconds))

(fn ConstructionScript
  (|CallParentFunction))

(fn GetTooltip
  (return 0))