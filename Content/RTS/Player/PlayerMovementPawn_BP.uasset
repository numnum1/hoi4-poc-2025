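; Player camera pawn for moving over the RTS map, with a spring-arm camera and wind audio.
; On restart it adds or removes the movement input mapping context depending on whether it is locally viewed.
; Tick applies movement from GetMove, scales wind volume with camera height and pitch with speed.
; Select, Move and Zoom events are empty; color-lookup province picking and radius-based zoom logic remain disconnected.
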(event EventTick
  (params (DeltaSeconds :type Float%20%28single-precision%29))
  (bind _windsoundeffect (Variables|Default|GetWindSoundEffect))
  (|CallParentFunction DeltaSeconds)
  (Audio|Components|Audio|SetVolumeMultiplier _windsoundeffect (Math|Float|MapRangeClamped (.Z (Math|Vector|BreakVector (Transformation|GetWorldLocation (Variables|Default|GetCamera)))) 0.0 2e+04 0.3 1.0) :!class /Script/Engine.AudioComponent)
  (Audio|Components|Audio|SetPitchMultiplier _windsoundeffect (Math|Float|MapRangeClamped (Math|Vector|VectorLength (Transformation|GetVelocity)) 0.0 2e+04 1.0 1.5))
  (Class|BAMapPawn|AddMovement DeltaSeconds (Input|EnhancedActionValues|GetMove)))

(event EventRestarted
  (bind _returnvalue (Game|GetPlayerController 0))
  (bind _returnvalue_2 (PlayerController|LocalPlayerSubsystems|GetEnhancedInputLocalPlayerSubsystem _returnvalue))
  (|CallParentFunction)
  (if (Pawn|IsLocallyViewed)
    (Input|AddMappingContext _returnvalue_2 "/Game/RTS/Player/DefaultMovementInputs_ICM.DefaultMovementInputs_ICM" 1 "(bIgnoreAllPressedKeysUntilRelease=True,bForceImmediately=False,bNotifyUserSettings=False)")
    (else
      (Utilities|IsValid _returnvalue
        (:Is%20Valid
          (Utilities|IsValid _returnvalue_2
            (:Is%20Valid
              (Input|RemoveMappingContext _returnvalue_2 "/Game/RTS/Player/DefaultMovementInputs_ICM.DefaultMovementInputs_ICM" "(bIgnoreAllPressedKeysUntilRelease=True,bForceImmediately=False,bNotifyUserSettings=False)"))))))))

(event EventSelect
  (params (HitResult :type Hit%20Result%20Structure) (UV :type Vector%202D%20Structure) (bHit :type Boolean)))

(event Input|EnhancedActionEvents|EnhancedInputActionZoom
  (params (ActionValue :type Float%20%28double-precision%29) (ElapsedSeconds :type Float%20%28double-precision%29) (TriggeredSeconds :type Float%20%28double-precision%29) (InputAction :type Input%20Action%20Object%20Reference :default "/Game/RTS/Player/Zoom.Zoom")))

(event Input|EnhancedActionEvents|EnhancedInputActionMove
  (params (ActionValue :type Vector :default "0, 0, 0") (ElapsedSeconds :type Float%20%28double-precision%29) (TriggeredSeconds :type Float%20%28double-precision%29) (InputAction :type Input%20Action%20Object%20Reference :default "/Game/RTS/Player/Move.Move")))

(fn ConstructionScript
  (|CallParentFunction)
  (Variables|Default|SetArmLength (Variables|/Script/Engine.SpringArmComponent|GetTargetArmLength (Variables|Default|GetSpringArm))))