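; RTS map actor that positions State_BP actors and colors provinces by map mode.
; BeginPlay indexes states by MapId, moves them to their province's unit position and binds repaint events that rewrite single LUT entries.
; UpdateMapWithCustomMode builds color entries from province history for political, demographic, geographic and state-debug modes, then rewrites the LUTs.
; State debug colors are deterministic hashes of state IDs; the province-subset update branch is disconnected.
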(event Custom|Repaint_Event
  (params (MapID :type Name) (Primary :type Color%20Structure) (Secondary :type Color%20Structure) (National :type Color%20Structure))
  (Class|BAMap|WritetoLUTs (Utilities|Array|MakeArray (Utilities|Struct|MakeDataLUT (.Color (Utilities|Struct|BreakProvinceMapDataGame (.Value (Utilities|Map|Find (Variables|Default|GetProvinceMapDataGame) MapID)))) Primary Secondary National)) false false))

(event EventBeginPlay
  (|CallParentFunction)
  (bind _outactors (Actor|GetAllActorsOfClass "/Game/RTS/State/State_BP.State_BP_C"))
  (for _array_element _outactors
    (Utilities|FlowControl|Sequence
      (:then_0
        (Utilities|Map|Add (Variables|Default|GetStates) (Variables|/Game/RTS/State/State_BP.State_BP_C|GetMapId _array_element) _array_element)
        (if (.ReturnValue (Utilities|Map|Find (Variables|Default|GetProvinceMapDataGame) (Variables|/Game/RTS/State/State_BP.State_BP_C|GetMapId _array_element)))
          (Transformation|SetActorLocation _array_element (Class|BAMap|UVtoLocation (.UnitPosition (Utilities|Struct|BreakProvinceMapDataGame (.Value (Utilities|Map|Find (Variables|Default|GetProvinceMapDataGame) (Variables|/Game/RTS/State/State_BP.State_BP_C|GetMapId _array_element)))))) false false)
          (else
            (Development|PrintString "State has no province"))))
      (:then_1
        (EventDispatchers|AssignRepaint _array_element (delegate Custom|Repaint_Event))))))

(fn ConstructionScript
  (|CallParentFunction))

(fn UpdateMap
  (params (MapMode :type E_DemoMapModes%20Enum :default "NewEnumerator4") (SpecificProvincesToUpdate :type Array%20of%20Names))
  (|CallParentFunction MapMode SpecificProvincesToUpdate)
  (return))

(fn UpdateMapwithCustomMode
  (params (MapMode :type E_DemoMapModes%20Enum :default "NewEnumerator4") (SpecificProvincesToUpdate :type Array%20of%20Names) (CustomMapMode :type %20Object%20Reference))
  (bind _countries (Variables|Default|GetCountries))
  (Variables|Default|SetMapMode MapMode)
  (LocalVariables|SetHistoryDataToUpdate (Variables|Default|GetProvinceHistoryData))
  (Utilities|FlowControl|Sequence
    (:then_0
      (switch Utilities|FlowControl|Switch|SwitchonE_DemoMapModes MapMode
        (:NewEnumerator0
          ;[0.2 0 1] Political
          (bind (_keypin _valuepin) (Utilities|Map|ForEachLoop(Map) (LocalVariables|GetHistoryDataToUpdate))
            (:then
              (if (.ReturnValue (Utilities|Map|Find (Variables|Default|GetProvinceMapDataGame) _keypin))
                (Utilities|Array|Add (LocalVariables|GetData) (Utilities|Struct|MakeDataLUT (Utilities|Struct|BreakProvinceMapDataGame (.Value (Utilities|Map|Find (Variables|Default|GetProvinceMapDataGame) _keypin))) (select (.ReturnValue (Utilities|Map|Find _countries (.Owner (Utilities|Struct|BreakStruct_DemoProvinceHistory _valuepin)))) (Variables|/BloodAnvil/Demo/Blueprints/Map/BP_Country.BP_Country_C|GetColor (.Value (Utilities|Map|Find _countries (.Owner (Utilities|Struct|BreakStruct_DemoProvinceHistory _valuepin))))) "") (select (.ReturnValue (Utilities|Map|Find _countries (.Controller (Utilities|Struct|BreakStruct_DemoProvinceHistory _valuepin)))) (Variables|/BloodAnvil/Demo/Blueprints/Map/BP_Country.BP_Country_C|GetColor (.Value (Utilities|Map|Find _countries (.Controller (Utilities|Struct|BreakStruct_DemoProvinceHistory _valuepin))))) (select (.ReturnValue (Utilities|Map|Find _countries (.Owner (Utilities|Struct|BreakStruct_DemoProvinceHistory _valuepin)))) (Variables|/BloodAnvil/Demo/Blueprints/Map/BP_Country.BP_Country_C|GetColor (.Value (Utilities|Map|Find _countries (.Owner (Utilities|Struct|BreakStruct_DemoProvinceHistory _valuepin))))) "")) (select (.ReturnValue (Utilities|Map|Find _countries (.Owner (Utilities|Struct|BreakStruct_DemoProvinceHistory _valuepin)))) (Variables|/BloodAnvil/Demo/Blueprints/Map/BP_Country.BP_Country_C|GetColor (.Value (Utilities|Map|Find _countries (.Owner (Utilities|Struct|BreakStruct_DemoProvinceHistory _valuepin))))) "")))))
            (:CompletedPin
              (LocalVariables|SetUpdateNational true))))
        (:NewEnumerator1
          ;[0.925 0.4408 0.3484] Cultural
          (bind (_keypin_2 _valuepin_2) (Utilities|Map|ForEachLoop(Map) (LocalVariables|GetHistoryDataToUpdate))
            (:then
              (if (.ReturnValue (Utilities|Map|Find (Variables|Default|GetProvinceMapDataGame) _keypin_2))
                (bind (_plurality_ _primary _secondary) (CallFunction|GetCultureMap (Utilities|Struct|BreakStruct_DemoProvinceHistory _valuepin_2)))
                (if _plurality_
                  (Utilities|Array|Add (LocalVariables|GetData) (Utilities|Struct|MakeDataLUT (Utilities|Struct|BreakProvinceMapDataGame (.Value (Utilities|Map|Find (Variables|Default|GetProvinceMapDataGame) _keypin_2))) (Utilities|Struct|BreakStruct_Culture (.Value (Utilities|Map|Find (Variables|Default|GetCultureData) _primary))) (Utilities|Struct|BreakStruct_Culture (.Value (Utilities|Map|Find (Variables|Default|GetCultureData) _secondary))) "(B=0,G=0,R=0,A=255)"))
                  (else
                    (Utilities|Array|Add (LocalVariables|GetData) (Utilities|Struct|MakeDataLUT (Utilities|Struct|BreakProvinceMapDataGame (.Value (Utilities|Map|Find (Variables|Default|GetProvinceMapDataGame) _keypin_2))) (Utilities|Struct|BreakStruct_Culture (.Value (Utilities|Map|Find (Variables|Default|GetCultureData) _primary))) (Utilities|Struct|BreakStruct_Culture (.Value (Utilities|Map|Find (Variables|Default|GetCultureData) _primary))) "(B=0,G=0,R=0,A=255)"))))))))
        (:NewEnumerator2
          ;[1 1 0.3] Religion
          (bind (_keypin_3 _valuepin_3) (Utilities|Map|ForEachLoop(Map) (LocalVariables|GetHistoryDataToUpdate))
            (:then
              (if (.ReturnValue (Utilities|Map|Find (Variables|Default|GetProvinceMapDataGame) _keypin_3))
                (bind (_plurality__2 _primary_2 _secondary_2) (CallFunction|GetReligionMap (Utilities|Struct|BreakStruct_DemoProvinceHistory _valuepin_3)))
                (if _plurality__2
                  (Utilities|Array|Add (LocalVariables|GetData) (Utilities|Struct|MakeDataLUT (Utilities|Struct|BreakProvinceMapDataGame (.Value (Utilities|Map|Find (Variables|Default|GetProvinceMapDataGame) _keypin_3))) (Utilities|Struct|BreakStruct_Religion (.Value (Utilities|Map|Find (Variables|Default|GetReligionData) _primary_2))) (Utilities|Struct|BreakStruct_Religion (.Value (Utilities|Map|Find (Variables|Default|GetReligionData) _secondary_2))) "(B=0,G=0,R=0,A=255)"))
                  (else
                    (Utilities|Array|Add (LocalVariables|GetData) (Utilities|Struct|MakeDataLUT (Utilities|Struct|BreakProvinceMapDataGame (.Value (Utilities|Map|Find (Variables|Default|GetProvinceMapDataGame) _keypin_3))) (Utilities|Struct|BreakStruct_Religion (.Value (Utilities|Map|Find (Variables|Default|GetReligionData) _primary_2))) (Utilities|Struct|BreakStruct_Religion (.Value (Utilities|Map|Find (Variables|Default|GetReligionData) _primary_2))) "(B=0,G=0,R=0,A=255)"))))))))
        (:NewEnumerator3
          ;[1 0.2488 0.2289] Literacy
          (bind (_keypin_4 _valuepin_4) (Utilities|Map|ForEachLoop(Map) (LocalVariables|GetHistoryDataToUpdate))
            (:then
              (if (.ReturnValue (Utilities|Map|Find (Variables|Default|GetProvinceMapDataGame) _keypin_4))
                (bind _literacy (CallFunction|GetLiteracy (Utilities|Struct|BreakStruct_DemoProvinceHistory _valuepin_4)))
                (Utilities|Array|Add (LocalVariables|GetData) (Utilities|Struct|MakeDataLUT (Utilities|Struct|BreakProvinceMapDataGame (.Value (Utilities|Map|Find (Variables|Default|GetProvinceMapDataGame) _keypin_4))) (Math|Conversions|ToColor(LinearColor) (Math|Color|Lerp(LinearColor) "(R=1.000000,G=0.000000,B=0.000000,A=1.000000)" "(R=0.000000,G=1.000000,B=0.000000,A=1.000000)" _literacy)) (Math|Conversions|ToColor(LinearColor) (Math|Color|Lerp(LinearColor) "(R=1.000000,G=0.000000,B=0.000000,A=1.000000)" "(R=0.000000,G=1.000000,B=0.000000,A=1.000000)" _literacy)) "(B=0,G=0,R=0,A=255)"))))))
        (:NewEnumerator9
          ;[0.2474 0.9402 1] State Debug Map Mode
          (bind (_keypin_5 _valuepin_5) (Utilities|Map|ForEachLoop(Map) (LocalVariables|GetHistoryDataToUpdate))
            (:then
              (if (.ReturnValue (Utilities|Map|Find (Variables|Default|GetProvinceMapDataGame) _keypin_5))
                (if (.ReturnValue (Utilities|Map|Find (Variables|Default|GetStateHistory) (Utilities|String|StringToName (Utilities|String|Append (Utilities|String|ToString(Name) (.State (Utilities|Struct|BreakProvinceMapDataGame (.Value (Utilities|Map|Find (Variables|Default|GetProvinceMapDataGame) _keypin_5))))) "_" (Utilities|String|ToString(Name) (Utilities|Struct|BreakStruct_DemoProvinceHistory _valuepin_5))))))
                  (Utilities|Array|Add (LocalVariables|GetData) (Utilities|Struct|MakeDataLUT (.Color (Utilities|Struct|BreakProvinceMapDataGame (.Value (Utilities|Map|Find (Variables|Default|GetProvinceMapDataGame) _keypin_5)))) (Math|Conversions|ToColor(LinearColor) (Utilities|Struct|MakeLinearColor (Math|Float|Fraction (Math|Float|Power (Math|Conversions|ToFloat(Integer) (Utilities|String|ToString(Name) (.State (Utilities|Struct|BreakProvinceMapDataGame (.Value (Utilities|Map|Find (Variables|Default|GetProvinceMapDataGame) _keypin_5)))))) 1.32178)) (Math|Float|Fraction (Math|Float|Power (Math|Conversions|ToFloat(Integer) (Utilities|String|ToString(Name) (.State (Utilities|Struct|BreakProvinceMapDataGame (.Value (Utilities|Map|Find (Variables|Default|GetProvinceMapDataGame) _keypin_5)))))) 1.201209)) (Math|Float|Fraction (Math|Float|Power (Math|Conversions|ToFloat(Integer) (Utilities|String|ToString(Name) (.State (Utilities|Struct|BreakProvinceMapDataGame (.Value (Utilities|Map|Find (Variables|Default|GetProvinceMapDataGame) _keypin_5)))))) 1.933928)) 1.0)) (select (.Split (Utilities|Struct|BreakStruct_DemoStateData (.Value (Utilities|Map|Find (Variables|Default|GetStateHistory) (Utilities|String|StringToName (Utilities|String|Append (Utilities|String|ToString(Name) (.State (Utilities|Struct|BreakProvinceMapDataGame (.Value (Utilities|Map|Find (Variables|Default|GetProvinceMapDataGame) _keypin_5))))) "_" (Utilities|String|ToString(Name) (Utilities|Struct|BreakStruct_DemoProvinceHistory _valuepin_5)))))))) (Utilities|Struct|BreakStruct_DemoCountryHistory (.Value (Utilities|Map|Find (Variables|Default|GetCountryData) (Utilities|Struct|BreakStruct_DemoProvinceHistory _valuepin_5)))) (Math|Conversions|ToColor(LinearColor) (Utilities|Struct|MakeLinearColor (Math|Float|Fraction (Math|Float|Power (Math|Conversions|ToFloat(Integer) (Utilities|String|ToString(Name) (.State (Utilities|Struct|BreakProvinceMapDataGame (.Value (Utilities|Map|Find (Variables|Default|GetProvinceMapDataGame) _keypin_5)))))) 1.32178)) (Math|Float|Fraction (Math|Float|Power (Math|Conversions|ToFloat(Integer) (Utilities|String|ToString(Name) (.State (Utilities|Struct|BreakProvinceMapDataGame (.Value (Utilities|Map|Find (Variables|Default|GetProvinceMapDataGame) _keypin_5)))))) 1.201209)) (Math|Float|Fraction (Math|Float|Power (Math|Conversions|ToFloat(Integer) (Utilities|String|ToString(Name) (.State (Utilities|Struct|BreakProvinceMapDataGame (.Value (Utilities|Map|Find (Variables|Default|GetProvinceMapDataGame) _keypin_5)))))) 1.933928)) 1.0))) "(B=0,G=0,R=0,A=255)")))))))
        (:NewEnumerator5
          ;[0.925 0.5138 0.2683] Climate
          (bind (_keypin_6 _valuepin_6) (Utilities|Map|ForEachLoop(Map) (LocalVariables|GetHistoryDataToUpdate))
            (:then
              (if (.ReturnValue (Utilities|Map|Find (Variables|Default|GetProvinceMapDataGame) _keypin_6))
                (if (.ReturnValue (Utilities|Map|Find (Variables|Default|GetClimateData) (Utilities|Struct|BreakStruct_DemoProvinceHistory _valuepin_6)))
                  (Utilities|Array|Add (LocalVariables|GetData) (Utilities|Struct|MakeDataLUT (Utilities|Struct|BreakProvinceMapDataGame (.Value (Utilities|Map|Find (Variables|Default|GetProvinceMapDataGame) _keypin_6))) (Utilities|Struct|BreakStruct_Climate (.Value (Utilities|Map|Find (Variables|Default|GetClimateData) (Utilities|Struct|BreakStruct_DemoProvinceHistory _valuepin_6)))) (Utilities|Struct|BreakStruct_Climate (.Value (Utilities|Map|Find (Variables|Default|GetClimateData) (Utilities|Struct|BreakStruct_DemoProvinceHistory _valuepin_6)))) "(B=0,G=0,R=0,A=255)")))))))
        (:NewEnumerator6
          ;[0.2188 0.1838 0.1472] Terrain
          (bind (_keypin_7 _valuepin_7) (Utilities|Map|ForEachLoop(Map) (LocalVariables|GetHistoryDataToUpdate))
            (:then
              (if (.ReturnValue (Utilities|Map|Find (Variables|Default|GetProvinceMapDataGame) _keypin_7))
                (if (.ReturnValue (Utilities|Map|Find (Variables|Default|GetTerrainData) (Utilities|Struct|BreakStruct_DemoProvinceHistory _valuepin_7)))
                  (Utilities|Array|Add (LocalVariables|GetData) (Utilities|Struct|MakeDataLUT (Utilities|Struct|BreakProvinceMapDataGame (.Value (Utilities|Map|Find (Variables|Default|GetProvinceMapDataGame) _keypin_7))) (Utilities|Struct|BreakStruct_Terrain (.Value (Utilities|Map|Find (Variables|Default|GetTerrainData) (Utilities|Struct|BreakStruct_DemoProvinceHistory _valuepin_7)))) (Utilities|Struct|BreakStruct_Terrain (.Value (Utilities|Map|Find (Variables|Default|GetTerrainData) (Utilities|Struct|BreakStruct_DemoProvinceHistory _valuepin_7)))) "(B=0,G=0,R=0,A=255)")))))))
        (:NewEnumerator7
          ;[0.08965 0.2708 0.08887] Vegetation
          (bind (_keypin_8 _valuepin_8) (Utilities|Map|ForEachLoop(Map) (LocalVariables|GetHistoryDataToUpdate))
            (:then
              (if (.ReturnValue (Utilities|Map|Find (Variables|Default|GetProvinceMapDataGame) _keypin_8))
                (if (.ReturnValue (Utilities|Map|Find (Variables|Default|GetVegetationData) (Utilities|Struct|BreakStruct_DemoProvinceHistory _valuepin_8)))
                  (Utilities|Array|Add (LocalVariables|GetData) (Utilities|Struct|MakeDataLUT (Utilities|Struct|BreakProvinceMapDataGame (.Value (Utilities|Map|Find (Variables|Default|GetProvinceMapDataGame) _keypin_8))) (Utilities|Struct|BreakStruct_Vegetation (.Value (Utilities|Map|Find (Variables|Default|GetVegetationData) (Utilities|Struct|BreakStruct_DemoProvinceHistory _valuepin_8)))) (Utilities|Struct|BreakStruct_Vegetation (.Value (Utilities|Map|Find (Variables|Default|GetVegetationData) (Utilities|Struct|BreakStruct_DemoProvinceHistory _valuepin_8)))) "(B=0,G=0,R=0,A=255)")))))))))
    (:then_1
      (Class|BAMap|WritetoLUTs (LocalVariables|GetData) true (LocalVariables|GetUpdateNational)))))

(fn FindStatebyId
  (params (Key :type Name%20%28by%20ref%29))
  (return (.Value (Utilities|Map|Find (Variables|Default|GetStates) Key))))

(fn GetStates
  (bind _values (Utilities|Map|Values (Variables|Default|GetStates)))
  (return _values))