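; Organization actor for the RTS, holding a replicated name, logo and list of position holders.
; RepNotify functions broadcast info-changed and position-holders-changed events whenever that state updates.
; AddPositionHolder appends to a copy and reassigns the whole array, so the change triggers its RepNotify.
; FindPositionById is an unimplemented stub returning a placeholder "Leader" position for any Id.
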(event EventBeginPlay)

(event Collision|EventActorBeginOverlap
  (params (OtherActor :type Actor%20Object%20Reference)))

(event EventTick
  (params (DeltaSeconds :type Float%20%28single-precision%29)))

(fn ConstructionScript)

(fn OnRepName
  (Default|CallOnInfoChanged))

(fn OnRepLogo
  (Default|CallOnInfoChanged))

(fn AddPositionHolder
  (params (NewItem :type Organization%20Position%20Holder%20F%20Structure%20%28by%20ref%29))
  (bind _output_get (LocalVariables|Set_Copy (Variables|Default|GetPositionHolders)))
  (Utilities|Array|Add _output_get NewItem)
  (Variables|Default|SetPositionHolders _output_get))

(fn GetName
  (return (Variables|Default|GetName)))

(fn GetLogo
  (return (Variables|Default|GetLogo)))

(fn OnRepPositionHolders
  (Default|CallOnPositionHoldersChanged))

(fn FindPositionbyId
  (params (Id :type Guid%20Structure))
  ;[0.15 0.15 0.15 0.5] TODO: Implement
  (return (Utilities|Struct|MakeOrganizationPosition_F Id "Leader" (Class|WidgetBlueprintLibrary|MakeBrushfromTexture "/Game/RTS/Organization/T_NNB.T_NNB"))))