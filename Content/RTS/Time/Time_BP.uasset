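; Replicated game clock for the RTS that holds a DateTime and a Speed value, with getters for both.
; On authority, Tick advances DateTime by DeltaSeconds times 3600, truncated to whole seconds, so roughly one game hour passes per real second.
; RepNotify handlers fire OnTimeChanged and OnSpeedChanged dispatchers.
; SetSpeed stores Speed, but the tick calculation uses a fixed rate and ignores it.
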(event Custom|SetSpeed
  (params (Speed :type Integer))
  (Variables|Default|SetSpeed Speed))

(event EventTick
  (params (DeltaSeconds :type Float%20%28single-precision%29))
  (Networking|SwitchHasAuthority
    (:Authority
      (Variables|Default|SetDateTime (+ (Variables|Default|GetDateTime) (Math|Timespan|MakeTimespan 0 0 0 (Math|Float|Truncate (* (* DeltaSeconds 6e+01) 6e+01))))))))

(fn ConstructionScript)

(fn OnRepDateTime
  (Default|CallOnTimeChanged))

(fn OnRepSpeed
  (Default|CallOnSpeedChanged))

(fn GetDateTime
  (return (Variables|Default|GetDateTime)))

(fn GetSpeed
  (return (Variables|Default|GetSpeed)))