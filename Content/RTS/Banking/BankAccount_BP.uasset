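; BankAccount_BP is a bank account in the RTS banking system, holding a balance and a Data record that includes an owner and an ID.
; Getters expose the balance and data, and SetBalance overwrites the balance without validation.
; The balance uses a RepNotify, which finds the BankAccountHolder_BP component on the owner and calls its balance-changed event with the account ID.
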(fn OnRepBalance
  (bind _data (Variables|Default|GetData))
  (bind (_id _owner) (Utilities|Struct|BreakBankAccountData_F _data))
  (Default|CallOnBalanceChanged (Actor|GetComponentbyClass _owner "/Game/RTS/Banking/BankAccountHolder_BP.BankAccountHolder_BP_C") _id))

(fn GetBalance
  (return (Variables|Default|GetBalance)))

(fn SetBalance
  (params (Balance :type Integer))
  (Variables|Default|SetBalance Balance))

(fn GetData
  (return (Variables|Default|GetData)))