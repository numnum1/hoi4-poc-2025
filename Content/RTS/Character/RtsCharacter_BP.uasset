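; RTS character Blueprint that holds a character's replicated identity: name, portrait, current state and positions held in organizations.
; Each property's RepNotify calls a change notification, with name and portrait sharing the info-changed one, and getters expose the values.
; Registering a new organization position appends it to the list and explicitly calls the change notification.
; The construction script recomputes the Build member.
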(fn ConstructionScript
  (Default|Recompute (Variables|Default|GetBuild)))

(fn OnRepName
  (Default|CallOnInfoChanged))

(fn OnRepPortrait
  (Default|CallOnInfoChanged))

(fn OnRepCurrentState
  (Default|CallOnCurrentStateChanged))

(fn GetName
  (return (Variables|Default|GetName)))

(fn GetPortrait
  (return (Variables|Default|GetPortrait)))

(fn GetCurrentState
  (return (Variables|Default|GetCurrentState)))

(fn OnRepHoldPositionsinOrganizations
  (Default|CallOnHoldPositionsinOrganiazationsChanged))

(fn RegisterNewHoldPositioninOrganization
  (params (NewItem :type Position%20in%20Organization%20F%20Structure%20%28by%20ref%29))
  (bind _output_get (LocalVariables|Set_New (Variables|Default|GetHoldPositionsInOrganizations)))
  (Utilities|Array|Add _output_get NewItem)
  (Variables|Default|SetHoldPositionsInOrganizations _output_get)
  (Default|CallOnHoldPositionsinOrganiazationsChanged))

(fn GetHoldPositionsinOrganizations
  (return (Variables|Default|GetHoldPositionsInOrganizations)))